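; Left-hand door Blueprint for the DesertTown content that swings a door mesh around its yaw axis with a timeline.
; A box overlap opens and closes a Gate, whose exit drives a FlipFlop that alternates playing and reversing the Open timeline.
; No event shown feeds the Gate's Enter input.
; The construction script applies the Door mesh and DoorMaterial variables to the component.
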(event OnComponentBeginOverlap(Box)
  (params (OverlappedComponent :type Primitive%20Component%20Object%20Reference) (OtherActor :type Actor%20Object%20Reference) (OtherComp :type Primitive%20Component%20Object%20Reference) (OtherBodyIndex :type Integer) (bFromSweep :type Boolean) (SweepResult :type Hit%20Result%20Structure%20%28by%20ref%29))
  (Utilities|FlowControl|Gate true ; enters at Open
    (:Exit
      (Utilities|FlowControl|FlipFlop
        (:A
          (bind _newtrack_1 (Timeline|Open Play)
            (:Update
              (Transformation|SetRelativeRotation (Variables|Default|GetSM_Door_arch_1) (Math|Rotator|MakeRotator 0.0 0.0 (.z _newtrack_1)) false false))))
        (:B
          (Timeline|Open Reverse))))))

(event OnComponentEndOverlap(Box)
  (params (OverlappedComponent :type Primitive%20Component%20Object%20Reference) (OtherActor :type Actor%20Object%20Reference) (OtherComp :type Primitive%20Component%20Object%20Reference) (OtherBodyIndex :type Integer))
  (Utilities|FlowControl|Gate true ; enters at Close
    (:Exit
      (Utilities|FlowControl|FlipFlop
        (:A
          (bind _newtrack_1 (Timeline|Open Play)
            (:Update
              (Transformation|SetRelativeRotation (Variables|Default|GetSM_Door_arch_1) (Math|Rotator|MakeRotator 0.0 0.0 (.z _newtrack_1)) false false))))
        (:B
          (Timeline|Open Reverse))))))

(fn ConstructionScript
  (bind _sm_door_arch_1 (Variables|Default|GetSM_Door_arch_1))
  (Components|StaticMesh|SetStaticMesh _sm_door_arch_1 (Variables|Default|GetDoor))
  (Rendering|Material|SetMaterial _sm_door_arch_1 0 (Variables|Default|GetDoorMaterial)))