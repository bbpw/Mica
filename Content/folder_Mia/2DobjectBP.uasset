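; A 2D billboard prop with a configurable flower material that pops up when the cave third-person character comes near.
; On BeginPlay it sinks its mesh below the placed position, then sphere begin and end overlaps raise and lower it with an eased MoveComponentTo, toggled by a Visible flag.
; Tick turns the mesh to face the player.
; SpecialTrigger disables both the overlap response and the facing.
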(event OnComponentBeginOverlap(Sphere)
  (params (OverlappedComponent :type Primitive%20Component%20Object%20Reference) (OtherActor :type Actor%20Object%20Reference) (OtherComp :type Primitive%20Component%20Object%20Reference) (OtherBodyIndex :type Integer) (bFromSweep :type Boolean) (SweepResult :type Hit%20Result%20Structure%20%28by%20ref%29))
  (Utilities|Casting|CastToThirdPersonCharacter_Cave OtherActor)
  (if (not (Variables|Default|GetSpecialTrigger))
    (if (not (Variables|Default|GetVisible))
      (Components|MoveComponentTo (Variables|Debug|GetStaticMeshComponent) (Variables|Default|GetLocation) (Transformation|GetWorldRotation (Variables|Debug|GetStaticMeshComponent)) true true (Variables|Default|GetDuration) false)
      (bind _output_get (Variables|Default|SetVisible (not (Variables|Default|GetVisible))))
      (if _output_get
        (Variables|Default|SetLocation (Variables|Default|GetDown))
        (else
          (Variables|Default|SetLocation (Variables|Default|GetUp)))))))

(event OnComponentEndOverlap(Sphere)
  (params (OverlappedComponent :type Primitive%20Component%20Object%20Reference) (OtherActor :type Actor%20Object%20Reference) (OtherComp :type Primitive%20Component%20Object%20Reference) (OtherBodyIndex :type Integer))
  (Utilities|Casting|CastToThirdPersonCharacter_Cave OtherActor)
  (if (not (Variables|Default|GetSpecialTrigger))
    (if (Variables|Default|GetVisible)
      (Components|MoveComponentTo (Variables|Debug|GetStaticMeshComponent) (Variables|Default|GetLocation) (Transformation|GetWorldRotation (Variables|Debug|GetStaticMeshComponent)) true true (Variables|Default|GetDuration) false)
      (bind _output_get (Variables|Default|SetVisible (not (Variables|Default|GetVisible))))
      (if _output_get
        (Variables|Default|SetLocation (Variables|Default|GetDown))
        (else
          (Variables|Default|SetLocation (Variables|Default|GetUp)))))))

(event EventBeginPlay
  (bind _staticmeshcomponent (Variables|Debug|GetStaticMeshComponent))
  (bind _relativelocation (Variables|/Script/Engine.SceneComponent|GetRelativeLocation _staticmeshcomponent))
  (Rendering|Material|SetMaterial (Variables|Default|GetPlane) 0 (Variables|Default|GetFlowerMaterial))
  (Variables|Default|SetUp (Variables|/Script/Engine.SceneComponent|GetRelativeLocation (Variables|Debug|GetStaticMeshComponent)))
  (bind _output_get (Variables|Default|SetDown (Math|Vector|MakeVector (.x _relativelocation) (.y _relativelocation) (- (.z _relativelocation) 1e+02))))
  (Variables|Default|SetLocation _output_get)
  (Variables|Default|SetVisible true)
  (Components|MoveComponentTo (Variables|Debug|GetStaticMeshComponent) (Variables|Default|GetLocation) (Transformation|GetWorldRotation (Variables|Debug|GetStaticMeshComponent)) true true (Variables|Default|GetDuration) false)
  (bind _output_get_2 (Variables|Default|SetVisible (not (Variables|Default|GetVisible))))
  (if _output_get_2
    (Variables|Default|SetLocation (Variables|Default|GetDown))
    (else
      (Variables|Default|SetLocation (Variables|Default|GetUp)))))

(event EventTick
  (params (DeltaSeconds :type Float%20%28single-precision%29))
  (if (not (Variables|Default|GetSpecialTrigger))
    (Transformation|SetWorldRotation (Variables|Debug|GetStaticMeshComponent) (Math|Rotator|FindLookatRotation (Transformation|GetWorldLocation (Variables|Debug|GetStaticMeshComponent)) (Transformation|GetActorLocation (Game|GetPlayerCharacter 0))) false false)))

(fn ConstructionScript)